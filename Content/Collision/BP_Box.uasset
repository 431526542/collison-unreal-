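; BP_Box is a collision test actor that reveals portals when its static mesh begins an overlap.
; On overlap, it hides the mesh, stops physics and collision, then unhides every BP_Portal found via GetAllActorsOfClass, without filtering the overlapping actor.
; Begin overlap, end overlap and hit events print the components and actors involved for debugging.
; BeginPlay logs the Portal array's contents, and a disconnected for-loop example never runs.
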(event OnComponentBeginOverlap(StaticMesh)
  (params (OverlappedComponent :type Primitive%20Component%20Object%20Reference) (OtherActor :type Actor%20Object%20Reference) (OtherComp :type Primitive%20Component%20Object%20Reference) (OtherBodyIndex :type Integer) (bFromSweep :type Boolean) (SweepResult :type Hit%20Result%20Structure%20%28by%20ref%29))
  (bind _staticmesh (Variables|Default|GetStaticMesh))
  ;[1 1 1] 이벤트를 추가하면 실험해보고 각각 어떤 기능을 하는지 실험해본다.
  (Development|PrintString (Utilities|String|Append "Begin Overlap - " "Overlapped Component - " (Utilities|GetDisplayName OverlappedComponent) ".Other Actor - " (Utilities|GetDisplayName OtherActor) ".Other Comp - " (Utilities|GetDisplayName OtherComp)) true true "(R=0.000000,G=0.660000,B=1.000000,A=1.000000)" 6e+01)
  ;[1 1 1] 투명화(피직스)처리 중단(컬리전) /순서 중요
  (Rendering|SetVisibility _staticmesh false false)
  (Physics|SetSimulatePhysics _staticmesh false)
  (Collision|SetCollisionEnabled _staticmesh "NoCollision")
  (bind _outactors (Actor|GetAllActorsOfClass "/Game/Collision/BP_Portal.BP_Portal_C"))
  (for _array_element _outactors
    (Rendering|SetActorHiddenInGame _array_element false)))

(event OnComponentEndOverlap(StaticMesh)
  (params (OverlappedComponent :type Primitive%20Component%20Object%20Reference) (OtherActor :type Actor%20Object%20Reference) (OtherComp :type Primitive%20Component%20Object%20Reference) (OtherBodyIndex :type Integer))
  ;[1 1 1] 이벤트를 추가하면 실험해보고 각각 어떤 기능을 하는지 실험해본다.
  (Development|PrintString (Utilities|String|Append "End Overlap - " "Overlapped Component - " (Utilities|GetDisplayName OverlappedComponent) ".Other Actor - " (Utilities|GetDisplayName OtherActor) ".Other Comp - " (Utilities|GetDisplayName OtherComp)) true true "(R=1.000000,G=0.002553,B=0.122234,A=1.000000)" 6e+01))

(event OnComponentHit(StaticMesh)
  (params (HitComponent :type Primitive%20Component%20Object%20Reference) (OtherActor :type Actor%20Object%20Reference) (OtherComp :type Primitive%20Component%20Object%20Reference) (NormalImpulse :type Vector :default "0, 0, 0") (Hit :type Hit%20Result%20Structure%20%28by%20ref%29))
  (Development|PrintString (Utilities|String|Append "Hit Component - " "Overlapped Component - " (Utilities|GetDisplayName HitComponent) ".Other Actor - " (Utilities|GetDisplayName OtherActor) ".Other Comp - " (Utilities|GetDisplayName OtherComp)) true true "(R=0.997971,G=1.000000,B=0.000484,A=1.000000)"))

(event EventBeginPlay
  (for (_array_element _array_index) (Variables|Default|GetPortal)
    (Development|PrintString (Utilities|String|Append "Loop Body Element Name :" (Utilities|GetDisplayName _array_element) ".Index : " (Utilities|String|ToString(Integer) _array_index)) true true "(R=0.000000,G=0.660000,B=1.000000,A=1.000000)" 6e+01))
  (Development|PrintString "Complate!!" true true "(R=0.000000,G=0.660000,B=1.000000,A=1.000000)" 6e+01))

(event Collision|EventActorBeginOverlap
  (params (OtherActor :type Actor%20Object%20Reference)))

(event EventTick
  (params (DeltaSeconds :type Float%20%28single-precision%29)))

(fn ConstructionScript)