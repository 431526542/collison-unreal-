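; BP_TimeLineMove moves its Sphere component back and forth along its relative X axis.
; On BeginPlay, if IsPlay is true, a timeline plays or reverses according to IsMoveRight, setting X to its value times EndPoint.
; Each finish flips the direction and re-enters that branch to form a continuous ping-pong.
; The Play function only sets IsPlay, which is checked only at BeginPlay.
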(event EventBeginPlay
  (if (Variables|Default|GetIsPlay)
    ;[1 1 1] 상태에따른 실행라인 방향 처리
    (if (Variables|Default|GetIsMoveRight) :!label _label
      (bind _value (Timeline|타임라인_0 Play)
        (:Update
          ;[1 1 1] 이동
          (Transformation|SetRelativeLocation (Variables|Default|GetSphere) (Math|Vector|MakeVector (* _value (Variables|Default|GetEndPoint)) 0.0 0.0) false false))
        (:Finished
          ;[1 1 1] 방향 조정
          (Variables|Default|SetIsMoveRight (not (Variables|Default|GetIsMoveRight)))
          (goto _label)))
      (else
        (Timeline|타임라인_0 Reverse)))))

(fn ConstructionScript)

(fn Play
  (params (IsPlay :type Boolean))
  (Variables|Default|SetIsPlay IsPlay))